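; Swordman character Blueprint that turns movement axis input into world-space character movement.
; The front/back and left/right axis events share one chain that builds an X/Y direction from axis input, with Y negated, for AddMovementInput.
; The same chain stores FrontSpeed and RightSpeed, exposed through getter functions.
; BeginPlay, Tick, overlap and the construction script are empty.
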(event `self.ReceiveBeginPlay`)

(event `InputAxis|FrontBackwardMovement`
  (params (AxisValue :type "Float (single-precision)"))
  (bind _returnvalue (* (stale `InputAxis|LeftRightMovement` AxisValue) -1.0))
  (`self.AddMovementInput` (`KismetMathLibrary.MakeVector` AxisValue _returnvalue) 1.0 :!label _label)
  (set `self.FrontSpeed` AxisValue)
  (set `self.RightSpeed` _returnvalue))

(event `self.ReceiveActorBeginOverlap`
  (params (OtherActor :type "Actor Object Reference")))

(event `InputAxis|LeftRightMovement`
  (params (AxisValue :type "Float (single-precision)"))
  (goto _label))

(event `self.ReceiveTick`
  (params (DeltaSeconds :type "Float (single-precision)")))

(fn `GetFrontSpeed`
  (returns (ret :type "Float (double-precision)"))
  (return (`self.FrontSpeed`)))

(fn `GetRightSpeed`
  (returns (ret :type "Float (double-precision)"))
  (return (`self.RightSpeed`)))

(fn `UserConstructionScript`)